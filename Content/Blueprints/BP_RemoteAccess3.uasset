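; BP_RemoteAccess3 is an interactable remote control that triggers three remote doors at once.
; On BeginPlay, nested GetAllActorsOfClass loops cast and store one reference each for BP_RemoteDoor, BP_RemoteDoor2 and BP_RemoteDoor3, keeping the last instance found.
; WasInteracted sets each stored door's Open flag to false, then calls its OpenDoorEvent.
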(event `self.ReceiveBeginPlay`
  ;[1 1 1] cast all doors
  (bind _outactors (`GameplayStatics.GetAllActorsOfClass` "/Game/Blueprints/BP_RemoteDoor2.BP_RemoteDoor2_C"))
  (for _array_element _outactors
    (bind _asbp_remote_door_2 (cast `/Game/Blueprints/BP_RemoteDoor2` _array_element))
    (set `self.RemoteDoor2` _asbp_remote_door_2)
    (bind _outactors_2 (`GameplayStatics.GetAllActorsOfClass` "/Game/Blueprints/BP_RemoteDoor3.BP_RemoteDoor3_C"))
    (for _array_element_2 _outactors_2
      (bind _asbp_remote_door_3 (cast `/Game/Blueprints/BP_RemoteDoor3` _array_element_2))
      (set `self.RemoteDoor3` _asbp_remote_door_3)
      (bind _outactors_3 (`GameplayStatics.GetAllActorsOfClass` "/Game/Blueprints/BP_RemoteDoor.BP_RemoteDoor_C"))
      (for _array_element_3 _outactors_3
        (bind _asbp_remote_door (cast `/Game/Blueprints/BP_RemoteDoor` _array_element_3))
        (set `self.RemoteDoor1` _asbp_remote_door)))))

(event `self.WasInteracted`
  (bind _remotedoor2 (`self.RemoteDoor2`))
  (bind _remotedoor1 (`self.RemoteDoor1`))
  (bind _remotedoor3 (`self.RemoteDoor3`))
  ;[1 1 1] open all doors
  (set `/Game/Blueprints/BP_RemoteDoor2.Open` false _remotedoor2)
  (set `/Game/Blueprints/BP_RemoteDoor.Open` false _remotedoor1)
  (set `/Game/Blueprints/BP_RemoteDoor3.Open` false _remotedoor3)
  (`/Game/Blueprints/BP_RemoteDoor2.OpenDoor_Event` _remotedoor2)
  (`/Game/Blueprints/BP_RemoteDoor.OpenDoor_Event` _remotedoor1)
  (`/Game/Blueprints/BP_RemoteDoor3.OpenDoor_Event` _remotedoor3))

(fn `UserConstructionScript`)