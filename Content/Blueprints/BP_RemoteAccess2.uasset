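; BP_RemoteAccess2 is an interactable remote control that operates three remote doors.
; On BeginPlay, nested GetAllActorsOfClass loops cache one instance each of BP_RemoteDoor, BP_RemoteDoor2 and BP_RemoteDoor3, keeping the last found.
; WasInteracted calls OpenDoorEvent on all three, then on authority only toggles the Open flag of RemoteDoor2 and RemoteDoor3 and forces RemoteDoor1's to false.
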(event `self.ReceiveBeginPlay`
  ;[1 1 1] cast all doors
  (bind _outactors (`GameplayStatics.GetAllActorsOfClass` "/Game/Blueprints/BP_RemoteDoor2.BP_RemoteDoor2_C"))
  (for _array_element _outactors
    (bind _asbp_remote_door_2 (cast `/Game/Blueprints/BP_RemoteDoor2` _array_element))
    (set `self.RemoteDoor2` _asbp_remote_door_2)
    (bind _outactors_2 (`GameplayStatics.GetAllActorsOfClass` "/Game/Blueprints/BP_RemoteDoor3.BP_RemoteDoor3_C"))
    (for _array_element_2 _outactors_2
      (bind _asbp_remote_door_3 (cast `/Game/Blueprints/BP_RemoteDoor3` _array_element_2))
      (set `self.RemoteDoor3` _asbp_remote_door_3)
      (bind _outactors_3 (`GameplayStatics.GetAllActorsOfClass` "/Game/Blueprints/BP_RemoteDoor.BP_RemoteDoor_C"))
      (for _array_element_3 _outactors_3
        (set `self.RemoteDoor1` _array_element_3)))))

(event `self.WasInteracted`
  (bind _remotedoor2 (`self.RemoteDoor2`))
  (bind _remotedoor3 (`self.RemoteDoor3`))
  (bind _remotedoor1 (`self.RemoteDoor1`))
  ;[1 1 1] open first and third door but close second one
  (`/Game/Blueprints/BP_RemoteDoor2.OpenDoor_Event` _remotedoor2)
  (`/Game/Blueprints/BP_RemoteDoor3.OpenDoor_Event` _remotedoor3)
  (`/Game/Blueprints/BP_RemoteDoor.OpenDoor_Event` _remotedoor1)
  (`/Engine/EditorBlueprintResources/ActorMacros.Switch Has Authority`
    (:`Authority`
      (set `/Game/Blueprints/BP_RemoteDoor3.Open` (not (`/Game/Blueprints/BP_RemoteDoor3.Open` _remotedoor3)) _remotedoor3)
      (set `/Game/Blueprints/BP_RemoteDoor2.Open` (not (`/Game/Blueprints/BP_RemoteDoor2.Open` _remotedoor2)) _remotedoor2)
      (set `/Game/Blueprints/BP_RemoteDoor.Open` false _remotedoor1))))

(fn `UserConstructionScript`)